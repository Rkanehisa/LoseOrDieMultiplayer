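; TrackMasterBP is a track piece Blueprint, apparently a base class, that knows its end point and the track piece that follows it.
; The construction script moves the NextTrackCollision component to the EndPoint's relative location.
; When that collision begins overlapping another TrackMasterBP, it stores that actor as NextTrack.
; GetAttachTransform exposes the EndPoint's world transform as the piece's attach point.
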(event OnComponentBeginOverlap(NextTrackCollision)
  (params (OverlappedComponent :type Primitive%20Component%20Object%20Reference) (OtherActor :type Actor%20Object%20Reference) (OtherComp :type Primitive%20Component%20Object%20Reference) (OtherBodyIndex :type Integer) (bFromSweep :type Boolean) (SweepResult :type Hit%20Result%20Structure%20%28by%20ref%29))
  (bind _astrack_master_bp (Utilities|Casting|CastToTrackMasterBP OtherActor))
  (Variables|Default|SetNextTrack _astrack_master_bp))

(event EventBeginPlay)

(event EventActorBeginOverlap
  (params (OtherActor :type Actor%20Object%20Reference)))

(event EventTick
  (params (DeltaSeconds :type Float%20%28single-precision%29)))

(fn ConstructionScript
  (Transformation|SetRelativeLocation (Variables|Default|GetNextTrackCollision) (Variables|/Script/Engine.SceneComponent|GetRelativeLocation (Variables|Default|GetEndPoint)) false false))

(fn GetAttachTransform
  (return (Transformation|GetWorldTransform (Variables|Default|GetEndPoint))))