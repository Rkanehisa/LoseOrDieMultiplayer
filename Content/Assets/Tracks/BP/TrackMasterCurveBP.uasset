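; Base track curve piece that prepares the car player for a turn and warns of its direction.
; When a car player overlaps the curve collision, it copies the integer Angle into the car's turn angle and enables turning.
; It then starts the car's curve HUD countdown and shows the right or left warning widget according to the sign of the angle.
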(event OnComponentBeginOverlap(SetCurveCollision)
  (params (OverlappedComponent :type Primitive%20Component%20Object%20Reference) (OtherActor :type Actor%20Object%20Reference) (OtherComp :type Primitive%20Component%20Object%20Reference) (OtherBodyIndex :type Integer) (bFromSweep :type Boolean) (SweepResult :type Hit%20Result%20Structure%20%28by%20ref%29))
  (bind _ascar_player_character (Utilities|Casting|CastToCarPlayerCharacter OtherActor))
  (CallFunction|SetPlayerVariables _ascar_player_character)
  (Default|CurveHudCountDown _ascar_player_character)
  (bind _ascurve_warnig_widget (Utilities|Casting|CastToCurveWarnigWidget (Variables|/Game/ThirdPersonBP/Blueprints/CarPlayerCharacter.CarPlayerCharacter_C|GetCurveHud _ascar_player_character)))
  (Math|Integer|CompareInt (Variables|Default|GetAngle) 0
    (:>
      (Widget|SetVisibility (Variables|/Game/Assets/UI/CurveWarnigWidget.CurveWarnigWidget_C|GetRightCurveWarning _ascurve_warnig_widget) "Visible"))
    (:<
      (Widget|SetVisibility (Variables|/Game/Assets/UI/CurveWarnigWidget.CurveWarnigWidget_C|GetLeftCurveWarning _ascurve_warnig_widget) "Visible"))))

(event EventBeginPlay)

(event EventActorBeginOverlap
  (params (OtherActor :type Actor%20Object%20Reference)))

(event EventTick
  (params (DeltaSeconds :type Float%20%28single-precision%29)))

(fn ConstructionScript
  (|CallParentFunction))

(fn SetPlayerVariables
  (params (CarPlayer :type Car%20Player%20Character%20Object%20Reference))
  (Variables|/Game/ThirdPersonBP/Blueprints/CarPlayerCharacter.CarPlayerCharacter_C|SetTurnAngle CarPlayer (Math|Conversions|ToFloat(Integer) (Variables|Default|GetAngle)))
  (Variables|/Game/ThirdPersonBP/Blueprints/CarPlayerCharacter.CarPlayerCharacter_C|SetCanTurn CarPlayer true))