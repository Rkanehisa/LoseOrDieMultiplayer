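; Floating barrier actor that bobs its static mesh vertically to give an idle hovering motion.
; On BeginPlay it runs a custom event that randomly picks one of six timelines and plays it from the start.
; Each timeline update adds its curve value as a relative Z offset, so movement accumulates per update rather than setting an absolute position.
; When a timeline finishes, the event calls itself again, looping indefinitely with varied animations.
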(event Custom|FloatingAnimation
  (bind _staticmesh (Variables|Default|GetStaticMesh))
  (bind _staticmesh_2 (Variables|Default|GetStaticMesh))
  ;[1 1 1] Switch Floating Animations
  (switch int (Math|Random|RandomIntegerinRange 0 5)
    (:0
      (bind _floatinganimationposition (Timeline|Animation1 PlayFromStart)
        (:Update
          (Transformation|AddRelativeLocation _staticmesh_2 (Math|Vector|MakeVector 0.0 0.0 _floatinganimationposition) false false))
        (:Finished
          (CallFunction|FloatingAnimation :!label _label))))
    (:1
      (bind _floatinganimationposition_2 (Timeline|Timeline_0 PlayFromStart)
        (:Update
          (Transformation|AddRelativeLocation _staticmesh_2 (Math|Vector|MakeVector 0.0 0.0 _floatinganimationposition_2) false false))
        (:Finished
          (goto _label))))
    (:2
      (bind _floatinganimationposition_3 (Timeline|Timeline_1 PlayFromStart)
        (:Update
          (Transformation|AddRelativeLocation _staticmesh_2 (Math|Vector|MakeVector 0.0 0.0 _floatinganimationposition_3) false false))
        (:Finished
          (goto _label))))
    (:3
      (bind _floatinganimationposition_4 (Timeline|Timeline_2 PlayFromStart)
        (:Update
          (Transformation|AddRelativeLocation _staticmesh (Math|Vector|MakeVector 0.0 0.0 _floatinganimationposition_4) false false))
        (:Finished
          (CallFunction|FloatingAnimation :!label _label_2))))
    (:4
      (bind _floatinganimationposition_5 (Timeline|Timeline_3 PlayFromStart)
        (:Update
          (Transformation|AddRelativeLocation _staticmesh (Math|Vector|MakeVector 0.0 0.0 _floatinganimationposition_5) false false))
        (:Finished
          (goto _label_2))))
    (:5
      (bind _floatinganimationposition_6 (Timeline|Timeline_4 PlayFromStart)
        (:Update
          (Transformation|AddRelativeLocation _staticmesh (Math|Vector|MakeVector 0.0 0.0 _floatinganimationposition_6) false false))
        (:Finished
          (goto _label_2))))))

(event EventBeginPlay
  (CallFunction|FloatingAnimation))

(event Collision|EventActorBeginOverlap
  (params (OtherActor :type Actor%20Object%20Reference)))

(event EventTick
  (params (DeltaSeconds :type Float%20%28single-precision%29)))

(fn ConstructionScript)