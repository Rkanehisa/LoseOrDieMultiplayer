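; RandomObstaclesArea is an actor that scatters a small random set of obstacles and arrow pickups or markers inside its Box volume.
; The Construction Script runs a short random-length loop, picking down arrow, up arrow, reverse arrow or obstacle cube each pass.
; Each helper adds a Child Actor Component at a random point in the box, with cubes also getting random yaw.
; All generation happens at construction, as the Event Graph is empty.
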(event EventBeginPlay)

(event Collision|EventActorBeginOverlap
  (params (OtherActor :type Actor%20Object%20Reference)))

(event EventTick
  (params (DeltaSeconds :type Float%20%28single-precision%29)))

(fn ConstructionScript
  (for _index (range 0 (Math|Random|RandomIntegerinRange 0 4))
    (switch int (Math|Random|RandomIntegerinRange 0 3)
      (:0
        (CallFunction|AddArrowDown))
      (:1
        (CallFunction|AddArrowUp))
      (:2
        (CallFunction|AddObstacleCube))
      (:3
        (CallFunction|AddReverseArrow)))))

(fn AddArrowDown
  (bind _box (Variables|Default|GetBox))
  (AddComponent|AddChildActorComponent false (Math|Transform|MakeTransform (Math|Random|RandomPointinBoundingBox (Variables|/Script/Engine.SceneComponent|GetRelativeLocation _box) (Variables|/Script/Engine.BoxComponent|GetBoxExtent _box)) "0, 0, 0" "1,1,1")))

(fn AddArrowUp
  (bind _box (Variables|Default|GetBox))
  (AddComponent|AddChildActorComponent false (Math|Transform|MakeTransform (Math|Random|RandomPointinBoundingBox (Variables|/Script/Engine.SceneComponent|GetRelativeLocation _box) (Variables|/Script/Engine.BoxComponent|GetBoxExtent _box)) "0, 0, 0" "1,1,1")))

(fn AddObstacleCube
  (bind _box (Variables|Default|GetBox))
  (AddComponent|AddChildActorComponent false (Math|Transform|MakeTransform (Math|Random|RandomPointinBoundingBox (Variables|/Script/Engine.SceneComponent|GetRelativeLocation _box) (Variables|/Script/Engine.BoxComponent|GetBoxExtent _box)) (Math|Rotator|MakeRotator 0.0 0.0 (Math|Random|RandomFloatinRange 0.0 359.0)) "1,1,1")))

(fn AddReverseArrow
  (bind _box (Variables|Default|GetBox))
  (AddComponent|AddChildActorComponent false (Math|Transform|MakeTransform (Math|Random|RandomPointinBoundingBox (Variables|/Script/Engine.SceneComponent|GetRelativeLocation _box) (Variables|/Script/Engine.BoxComponent|GetBoxExtent _box)) "0, 0, 0" "1,1,1")))